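; BP_AimingCharacter is a player character that moves, looks around and aims a rifle, with the aiming passed on to its Animation Blueprint.
; On BeginPlay it caches ABP_AimingCharacter from the mesh, then spawns BP_AimingRifle and snaps it to a mesh socket.
; The rifle calculates its sight transforms and hands the result to the AnimBP.
; Pressing Aim calls the AnimBP's Aim event.
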(event `self.ReceiveBeginPlay`
  (`self.RefToAnimBP`)
  (`self.AddGun`))

(event `InputAxis|MoveForward`
  (params (AxisValue :type "Float (single-precision)"))
  (`self.AddMovementInput` (`self.GetActorForwardVector`) AxisValue))

(event `InputAxis|MoveRight`
  (params (AxisValue :type "Float (single-precision)"))
  (`self.AddMovementInput` (`self.GetActorRightVector`) AxisValue))

(event `InputAxis|Turn`
  (params (AxisValue :type "Float (single-precision)"))
  (`self.AddControllerYawInput` AxisValue))

(event `InputAxis|LookUp`
  (params (AxisValue :type "Float (single-precision)"))
  (`self.AddControllerPitchInput` AxisValue))

(event `InputAction|Aim`
  (params (Key :type "Key Structure"))
  (:`Pressed`
    (`self.Aim`)))

(event `RefToAnimBP`
  (bind _asabp_aiming_character (cast `/Game/Geometry/Characters/U4_Mannequin/Animations/ABP_AimingCharacter` (`SkeletalMeshComponent.GetAnimInstance` (`self.Mesh`))))
  (set `self.AnimBP` _asabp_aiming_character))

(event `AddGun`
  (bind _returnvalue (`|SpawnActorFromClass` "/Game/Blueprints/Weapons/BP_AimingRifle.BP_AimingRifle_C" (`KismetMathLibrary.MakeTransform` (0.0 0.0 0.0)) "Undefined" "OverrideRootScale" self null))
  (set `self.Gun` _returnvalue)
  (`SceneComponent.K2_AttachToComponent` (`/Game/Blueprints/Weapons/BP_AimingRifle.Main` (`self.Gun`)) (`self.Mesh`) "Example_Socket" "SnapToTarget" "SnapToTarget" "KeepWorld" true)
  (`/Game/Blueprints/Weapons/BP_AimingRifle.CalcSightsTransforms` (`self.Gun`))
  (`/Game/Geometry/Characters/U4_Mannequin/Animations/ABP_AimingCharacter.NewSightTransform` (`self.AnimBP`) (`/Game/Blueprints/Weapons/BP_AimingRifle.SightTransform` (`self.Gun`))))

(event `Aim`
  (`/Game/Geometry/Characters/U4_Mannequin/Animations/ABP_AimingCharacter.Aim` (`self.AnimBP`)))

(fn `UserConstructionScript`)