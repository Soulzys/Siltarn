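; Rifle Blueprint that computes a sight alignment transform for aiming down its optic.
; CalcSightsTransforms casts the instigator to BP_AimingCharacter and expresses the OpticAimpoint socket relative to the character's hand_r socket.
; It stores that location and rotation in SightTransform, puts the negated inverse-relative X offset plus DistanceFromCamera into X scale, and prints the result.
; The event graph and construction script are empty.
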(fn `CalcSightsTransforms`
  (locals (Character :type "/Game/Blueprints/Characters/BP_AimingCharacter Object Reference"))
  (bind _returnvalue (`SceneComponent.GetSocketTransform` (`self.Main`) "OpticAimpoint" "RTS_World"))
  (bind _returnvalue_2 (`SceneComponent.GetSocketTransform` (`Character.Mesh` (`local.Character`)) "hand_r" "RTS_World"))
  (bind (_returnvalue_location _returnvalue_rotation) (`KismetMathLibrary.BreakTransform` (`KismetMathLibrary.MakeRelativeTransform` _returnvalue _returnvalue_2)))
  (bind _asbp_aiming_character (cast `/Game/Blueprints/Characters/BP_AimingCharacter` (`self.GetInstigator`)))
  (set `local.Character` _asbp_aiming_character)
  (bind _output_get (set `self.SightTransform` (`KismetMathLibrary.MakeTransform` _returnvalue_location _returnvalue_rotation (`KismetMathLibrary.MakeVector` (+ (* -1 (.x (.location (`KismetMathLibrary.MakeRelativeTransform` _returnvalue_2 _returnvalue)))) (`self.DistanceFromCamera`)) 1.0 1.0))))
  (`KismetSystemLibrary.PrintString` (`KismetStringLibrary.Conv_TransformToString` _output_get) true true (struct :`G` 0.66 :`B` 1.0 :`A` 1.0) 10.0))

(fn `UserConstructionScript`)